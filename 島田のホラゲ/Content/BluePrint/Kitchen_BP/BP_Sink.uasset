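; BP_Sink is a kitchen sink whose running water toggles on and off each time its Gimmick event fires.
; Gimmick requires the last actor to overlap the Interact component to be a Character, then a FlipFlop alternates between on and off.
; Timelines play or reverse to scale the water mesh and splash particles.
; After a short delay, it spawns an attenuated running sound, or stops that and spawns a shut-off sound.
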(event OnComponentBeginOverlap(Interact)
  (params (OverlappedComponent :type Primitive%20Component%20Object%20Reference) (OtherActor :type Actor%20Object%20Reference) (OtherComp :type Primitive%20Component%20Object%20Reference) (OtherBodyIndex :type Integer) (bFromSweep :type Boolean) (SweepResult :type Hit%20Result%20Structure%20%28by%20ref%29))
  ;[1 1 1] レバーに触れているか
  (bind _output_get (Variables|Default|SetOverlap_Actor OtherActor)))

(event EventGimmick
  (Utilities|Casting|CastToCharacter (stale OnComponentBeginOverlap(Interact) _output_get))
  (Utilities|FlowControl|FlipFlop
    (:A
      (Utilities|FlowControl|Sequence
        (:then_0
          ;[1 1 1] 水の表示、非表示
          (bind _0_0_0375 (Timeline|Water Play)
            (:Update
              (Transformation|SetRelativeScale3D (Variables|Default|GetWaterA) (Math|Vector|MakeVector _0_0_0375 _0_0_0375 0.607161)))))
        (:then_1
          (bind _0_0_1325 (Timeline|Splash！ Play)
            (:Update
              (Transformation|SetRelativeScale3D (Variables|Default|GetParticleSystem) (Math|Vector|MakeVector _0_0_1325 _0_0_1325 _0_0_1325)))))
        (:then_2
          ;[1 1 1] 音を出す
          (Utilities|FlowControl|Delay 0.2)
          (Variables|Default|SetSound_Set "/Game/SoundEffect/Water_HandSink.Water_HandSink")
          (bind _returnvalue (Audio|SpawnSoundatLocation (Variables|Default|GetSound_Set) (Transformation|GetSocketLocation (Variables|Default|GetWaterA) "None") "0, 0, 0" 0.1 1.0 0.0 "/Game/SoundEffect/Sound_Attenuation/SA_Sink_Water.SA_Sink_Water" 0 :!label _label))
          (Variables|Default|SetSound _returnvalue))))
    (:B
      (Utilities|FlowControl|Sequence
        (:then_0
          (Timeline|Water Reverse))
        (:then_1
          (Timeline|Splash！ Reverse))
        (:then_2
          (Utilities|FlowControl|Delay 0.2)
          (Audio|Components|Audio|Stop (Variables|Default|GetSound))
          (Variables|Default|SetSound_Set "/Game/SoundEffect/Water_HandSink_Stop.Water_HandSink_Stop")
          (goto _label))))))

(fn ConstructionScript)