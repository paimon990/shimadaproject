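; Refrigerator door Blueprint for the kitchen that swings open and closed when its DoorOpen event fires.
; It remembers the overlapping actor and only responds if that actor is a TestCharacter.
; A FlipFlop plays or reverses a timeline that adds yaw to the rotation captured at BeginPlay, with collision disabled during the swing.
; A DoOnce prints an unlock message; the GameFlag reference cached on overlap is never read here.
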(event EventDoorOpen
  (bind _default_rotation (Variables|Default|GetDefault_Rotation))
  ;[1 1 1] 誰がOpenイベントを始めたのか
  (Utilities|Casting|CastToTestCharacter (Variables|Default|GetIntract_Character))
  (Utilities|FlowControl|FlipFlop
    (:A
      (bind _0__90 (Timeline|ドアの角度調整 Play)
        (:Update
          ;[1 1 1] コリジョン設定
          (Collision|SetActorEnableCollision false))
        (:Finished
          (Collision|SetActorEnableCollision true)))
      ;[1 1 1] 現在の角度に合わせて+する
      (Transformation|SetActorRelativeRotation (Math|Rotator|MakeRotator (.roll _default_rotation) (.pitch _default_rotation) (+ (.yaw _default_rotation) _0__90)))
      (Utilities|FlowControl|DoOnce false
        (:Completed
          (Development|PrintString "UnLocked!!!"))))
    (:B
      (Timeline|ドアの角度調整 Reverse))))

(event EventBeginPlay
  ;[1 1 1] 本来の角度
  (Variables|Default|SetDefault_Rotation (Transformation|GetActorRotation)))

(event Collision|EventActorEndOverlap
  (params (OtherActor :type Actor%20Object%20Reference))
  ;[1 1 1] 接触したキャラを覚える
  (Variables|Default|SetIntract_Character 0))

(event Collision|EventActorBeginOverlap
  (params (OtherActor :type Actor%20Object%20Reference))
  ;[1 1 1] 接触したキャラを覚える
  (Variables|Default|SetIntract_Character OtherActor)
  (bind _asgame_flag (Utilities|Casting|CastToGameFlag (Game|GetGameInstance)))
  (Variables|Default|SetAs%20Game%20Flag _asgame_flag))

(fn ConstructionScript
  (|CallParentFunction))