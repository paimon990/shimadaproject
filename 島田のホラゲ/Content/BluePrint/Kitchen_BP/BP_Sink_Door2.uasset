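; Kitchen sink double-door actor that swings open and closed when DoorOpen is called while a TestCharacter is stored from overlap.
; A FlipFlop alternately plays and reverses a timeline that yaws two cubes in mirrored directions, based on the actor's starting rotation.
; Actor collision is disabled during the swing and restored when the timeline finishes.
; Overlap also caches the GameFlag game instance, which is otherwise unused here.
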(event EventDoorOpen
  (bind _default_rotation (Variables|Default|GetDefault_Rotation))
  ;[1 1 1] 誰がOpenイベントを始めたのか
  (Utilities|Casting|CastToTestCharacter (Variables|Default|GetIntract_Character))
  (Utilities|FlowControl|FlipFlop
    (:A
      (Variables|Default|SetOpened true)
      (bind __90_0 (Timeline|ドアの角度調整 Play) ; 設置角度によって調整必須
        (:Update
          ;[1 1 1] コリジョン設定
          (Collision|SetActorEnableCollision false))
        (:Finished
          (Collision|SetActorEnableCollision true)))
      (Utilities|FlowControl|Sequence
        (:then_0
          ;[1 1 1] 現在の角度に合わせて+する
          (Transformation|SetRelativeRotation (Variables|Default|GetCube) (Math|Rotator|MakeRotator (.roll _default_rotation) (.pitch _default_rotation) (+ (.yaw _default_rotation) __90_0)) false false))
        (:then_1
          (Transformation|SetRelativeRotation (Variables|Default|GetCube1) (Math|Rotator|MakeRotator (.roll _default_rotation) (.pitch _default_rotation) (* (- (+ (.yaw _default_rotation) __90_0) 1.8e+02) -1.0)) false false))))
    (:B
      (Variables|Default|SetOpened false)
      (Timeline|ドアの角度調整 Reverse))))

(event EventBeginPlay
  ;[1 1 1] 本来の角度
  (Variables|Default|SetDefault_Rotation (Transformation|GetActorRotation)))

(event Collision|EventActorEndOverlap
  (params (OtherActor :type Actor%20Object%20Reference))
  ;[1 1 1] 接触したキャラを覚える
  (Variables|Default|SetIntract_Character 0))

(event Collision|EventActorBeginOverlap
  (params (OtherActor :type Actor%20Object%20Reference))
  ;[1 1 1] 接触したキャラを覚える
  (Variables|Default|SetIntract_Character OtherActor)
  (bind _asgame_flag (Utilities|Casting|CastToGameFlag (Game|GetGameInstance)))
  (Variables|Default|SetAs%20Game%20Flag _asgame_flag))

(fn ConstructionScript
  (|CallParentFunction))