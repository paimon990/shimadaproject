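; Interactive glass door for the living-room set that swings open and closed on alternate DoorOpen calls.
; Overlap tracks the interacting character and caches the GameFlag game instance; DoorOpen requires that character to be a TestCharacter.
; A FlipFlop plays or reverses a timeline that adds yaw to the rotation saved at BeginPlay, with actor collision disabled during the swing and restored on finish.
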(event EventDoorOpen
  (bind _default_rotation (Variables|Default|GetDefault_Rotation))
  (Utilities|Casting|CastToTestCharacter (Variables|Default|GetIntract_Character))
  (Utilities|FlowControl|FlipFlop
    (:A
      (Variables|Default|SetOpened true)
      (bind _0__90 (Timeline|ドアの角度調整 Play) ; 角度を手作業で設定必須
        (:Update
          (Collision|SetActorEnableCollision false))
        (:Finished
          (Collision|SetActorEnableCollision true)))
      (Transformation|SetActorRotation (Math|Rotator|MakeRotator (.roll _default_rotation) (.pitch _default_rotation) (+ _0__90 (.yaw _default_rotation)))))
    (:B
      (Variables|Default|SetOpened false)
      (Timeline|ドアの角度調整 Reverse))))

(event EventBeginPlay
  ;[1 1 1] 本来の角度
  (Variables|Default|SetDefault_Rotation (Transformation|GetActorRotation)))

(event Collision|EventActorEndOverlap
  (params (OtherActor :type Actor%20Object%20Reference))
  ;[1 1 1] 接触したキャラを覚える
  (Variables|Default|SetIntract_Character 0))

(event Collision|EventActorBeginOverlap
  (params (OtherActor :type Actor%20Object%20Reference))
  ;[1 1 1] 接触したキャラを覚える
  (Variables|Default|SetIntract_Character OtherActor)
  (bind _asgame_flag (Utilities|Casting|CastToGameFlag (Game|GetGameInstance)))
  (Variables|Default|SetAs%20Game%20Flag _asgame_flag))

(fn ConstructionScript
  (|CallParentFunction))