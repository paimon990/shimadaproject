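; Hinged door that a player character (TestCharacter) toggles open and closed, and that BP_Creature can open.
; Overlap records the interacting actor; DoorOpen flip-flops a yaw timeline offset from the starting rotation, disabling collision while it moves.
; Opening also turns the knob Sphere, and DoOnce-plus-Delay gates debounce the open and close sounds.
; DoorOpenC plays the swing after a short delay when the flip-flop reads closed, without toggling it.
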(event EventDoorOpen
  (bind _sphere (Variables|Default|GetSphere))
  (bind _default_rotation (Variables|Default|GetDefault_Rotation))
  ;[1 1 1] 誰がOpenイベントを始めたのか
  (Utilities|Casting|CastToTestCharacter (Variables|Default|GetIntract_Character))
  (bind _isa (Utilities|FlowControl|FlipFlop)
    (:A
      (Utilities|FlowControl|Sequence
        (:then_0
          ;[1 1 1] ドアの開閉
          (bind _0_90 (Timeline|ドアの角度調整 Play) ; 角度を手作業で設定必須
            (:Update
              (Collision|SetActorEnableCollision false))
            (:Finished
              (Collision|SetActorEnableCollision true)))
          (Transformation|SetActorRotation (Math|Rotator|MakeRotator (.roll _default_rotation) (.pitch _default_rotation) (+ _0_90 (.yaw _default_rotation)))))
        (:then_1
          ;[1 1 1] ドアノブ回転
          (bind _0_90_2 (Timeline|タイムライン_0 PlayFromStart)
            (:Update
              (Transformation|SetRelativeRotation _sphere (Math|Rotator|MakeRotator _0_90_2 0.0 -1.8e+02) false false)
              (Utilities|FlowControl|DoOnce false :!label _label
                (:Completed
                  (Audio|SpawnSoundatLocation "/Game/SoundEffect/Free_SE/Door_Open_and_Close_Sound_tumeawase_06a.Door_Open_and_Close_Sound_tumeawase_06a" (Transformation|GetSocketLocation _sphere "None") "0, 0, 0" 1.0 1.0 0.0 "/Game/SoundEffect/Sound_Attenuation/SA_Door_Sound.SA_Door_Sound" 0)
                  (Utilities|FlowControl|Delay 2.0)
                  (goto _label Reset))))))))
    (:B
      (Utilities|FlowControl|Sequence
        (:then_0
          (Timeline|ドアの角度調整 Reverse))
        (:then_1
          ;[1 1 1] ドア閉まる音
          (Utilities|FlowControl|DoOnce false :!label _label_2
            (:Completed
              (Utilities|FlowControl|Delay 0.35)
              (Audio|SpawnSoundatLocation "/Game/SoundEffect/Free_SE/Door_Open_and_Close_Sound_tumeawase_06b.Door_Open_and_Close_Sound_tumeawase_06b" (Transformation|GetSocketLocation (Variables|Default|GetSphere) "None") "0, 0, 0" 1.0 1.0 0.0 "/Game/SoundEffect/Sound_Attenuation/SA_Door_Sound.SA_Door_Sound" 0)
              (Utilities|FlowControl|Delay 2.0)
              (goto _label_2 Reset))))))))

(event EventBeginPlay
  ;[1 1 1] 本来の角度
  (Variables|Default|SetDefault_Rotation (Transformation|GetActorRotation)))

(event Collision|EventActorEndOverlap
  (params (OtherActor :type Actor%20Object%20Reference))
  ;[1 1 1] 接触したキャラを覚える
  (Variables|Default|SetIntract_Character 0))

(event EventDoorOpenC
  (bind _default_rotation (Variables|Default|GetDefault_Rotation))
  ;[1 1 1] 誰がOpenイベントを始めたのか
  (Utilities|FlowControl|Delay 0.2) ; 必須
  (Utilities|Casting|CastToBP_Creature (Variables|Default|GetIntract_Character))
  (if (not (stale EventDoorOpen _isa))
    ;[1 1 1] ドアの開閉
    (bind _0_90 (Timeline|ドアの角度調整 Play) ; 角度を手作業で設定必須
      (:Update
        (Collision|SetActorEnableCollision false))
      (:Finished
        (Collision|SetActorEnableCollision true)))
    (Transformation|SetActorRotation (Math|Rotator|MakeRotator (.roll _default_rotation) (.pitch _default_rotation) (+ _0_90 (.yaw _default_rotation))))))

(event Collision|EventActorBeginOverlap
  (params (OtherActor :type Actor%20Object%20Reference))
  ;[1 1 1] 接触したキャラを覚える
  (Variables|Default|SetIntract_Character OtherActor)
  (bind _asgame_flag (Utilities|Casting|CastToGameFlag (Game|GetGameInstance)))
  (Variables|Default|SetAs%20Game%20Flag _asgame_flag))

(fn ConstructionScript
  (|CallParentFunction))