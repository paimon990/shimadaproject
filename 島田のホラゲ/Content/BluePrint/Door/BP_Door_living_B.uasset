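; Living-room door Blueprint that plays a locked-door sound and animates its parts when DoorOpen is called.
; Four timelines run together, rolling the two Sphere components with a rattle curve and yawing the two Cube components.
; A DoOnce blocks repeat triggers, with a sound reset called after a short delay to re-arm it.
; BeginPlay stores the actor's starting rotation, which the graph never reads.
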(event Custom|Sound_Reset
  (Utilities|FlowControl|DoOnce false) ; enters at Reset
)

(event EventDoorOpen
  (Utilities|FlowControl|DoOnce false
    (:Completed
      (Utilities|FlowControl|Sequence
        (:then_0
          (Audio|SpawnSoundatLocation "/Game/SoundEffect/Free_SE/Door_Locked.Door_Locked" (Transformation|GetSocketLocation (Variables|Default|GetDefaultSceneRoot) "None") "0, 0, 0" 1.0 1.0 0.0 "/Game/SoundEffect/Sound_Attenuation/SA_Door_Sound.SA_Door_Sound" 0)
          (Utilities|FlowControl|Delay 1.5)
          (CallFunction|SoundReset))
        (:then_1
          (bind _ガチャガチャ (Timeline|タイムライン_0 PlayFromStart)
            (:Update
              (Transformation|SetRelativeRotation (Variables|Components|GetSphere) (Math|Rotator|MakeRotator _ガチャガチャ 0.0 0.0) false false))))
        (:then_2
          (bind _ガチャガチャ_2 (Timeline|タイムライン_1 PlayFromStart)
            (:Update
              (Transformation|SetRelativeRotation (Variables|Components|GetSphere1) (Math|Rotator|MakeRotator _ガチャガチャ_2 0.0 0.0) false false))))
        (:then_3
          (Utilities|FlowControl|Sequence
            (:then_0
              (bind _0_90 (Timeline|タイムライン_2 PlayFromStart)
                (:Update
                  (Transformation|SetRelativeRotation (Variables|Components|GetCube) (Math|Rotator|MakeRotator 0.0 0.0 _0_90) false false))))
            (:then_1
              (bind _0_90_2 (Timeline|タイムライン_3 PlayFromStart)
                (:Update
                  (Transformation|SetRelativeRotation (Variables|Components|GetCube1) (Math|Rotator|MakeRotator 0.0 0.0 _0_90_2) false false))))))))))

(event EventBeginPlay
  ;[1 1 1] 本来の角度
  (Variables|Default|SetDefault_Rotation (Transformation|GetActorRotation)))

(fn ConstructionScript
  (|CallParentFunction))