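; Kitchen door that the player toggles open and shut with a key, and that a creature can open once unlocked.
; Overlap records the interacting character, and GameInstance flags hold key ownership and unlocked state.
; DoorOpen flip-flops a timeline that adds yaw to the starting rotation, disabling collision while it moves.
; DoorOpenC, after a short delay, plays that timeline for BP_Creature if the door is unlocked and not marked open.
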(event EventDoorOpen
  (bind _default_rotation (Variables|Default|GetDefault_Rotation))
  ;[1 1 1] 誰がOpenイベントを始めたのか
  (Utilities|Casting|CastToTestCharacter (Variables|Default|GetIntract_Character))
  ;[1 1 1] 鍵を所有しているか否か
  (if (Variables|/Game/BluePrint/GameFlag/GameFlag.GameFlag_C|GetKey_Kitchen_Got (Variables|Default|GetAs%20Game%20Flag))
    ;[1 1 1] 解除済みフラグ
    (Variables|/Game/BluePrint/GameFlag/GameFlag.GameFlag_C|SetDoor_Kitchen_Unlocked (Variables|Default|GetAs%20Game%20Flag) true)
    (Utilities|FlowControl|FlipFlop
      (:A
        (Variables|Default|SetOpened true)
        (bind _0_90 (Timeline|ドアの角度調整 Play)
          (:Update
            ;[1 1 1] コリジョン設定
            (Collision|SetActorEnableCollision false))
          (:Finished
            (Collision|SetActorEnableCollision true)))
        ;[1 1 1] 現在の角度に合わせて+する
        (Transformation|SetActorRelativeRotation (Math|Rotator|MakeRotator (.roll _default_rotation) (.pitch _default_rotation) (+ (.yaw _default_rotation) _0_90)))
        (Utilities|FlowControl|DoOnce false
          (:Completed
            (Development|PrintString "UnLocked!!!"))))
      (:B
        (Variables|Default|SetOpened false)
        (Timeline|ドアの角度調整 Reverse)))
    (else
      (Development|PrintString "Locked!!!"))))

(event EventDoorOpenC
  (bind _default_rotation (Variables|Default|GetDefault_Rotation))
  ;[1 1 1] 誰がOpenイベントを始めたのか
  (Utilities|FlowControl|Delay 0.2) ; 必須
  (Utilities|Casting|CastToBP_Creature (Variables|Default|GetIntract_Character))
  ;[1 1 1] 開錠済みか判断
  (if (Variables|/Game/BluePrint/GameFlag/GameFlag.GameFlag_C|GetDoor_Kitchen_Unlocked (Variables|Default|GetAs%20Game%20Flag))
    (if (not (Variables|Default|GetOpened))
      (bind _0_90 (Timeline|ドアの角度調整 Play)
        (:Update
          ;[1 1 1] コリジョン設定
          (Collision|SetActorEnableCollision false))
        (:Finished
          (Collision|SetActorEnableCollision true)))
      ;[1 1 1] 現在の角度に合わせて+する
      (Transformation|SetActorRelativeRotation (Math|Rotator|MakeRotator (.roll _default_rotation) (.pitch _default_rotation) (+ (.yaw _default_rotation) _0_90)))
      (Utilities|FlowControl|DoOnce false
        (:Completed
          (Development|PrintString "UnLocked!!!"))))))

(event EventBeginPlay
  ;[1 1 1] 本来の角度
  (bind _output_get (Variables|Default|SetDefault_Rotation (Transformation|GetActorRotation)))
  (Development|PrintString (Utilities|String|ToString(Rotator) _output_get)))

(event Collision|EventActorEndOverlap
  (params (OtherActor :type Actor%20Object%20Reference))
  ;[1 1 1] 接触したキャラを覚える
  (Variables|Default|SetIntract_Character 0))

(event Collision|EventActorBeginOverlap
  (params (OtherActor :type Actor%20Object%20Reference))
  ;[1 1 1] 接触したキャラを覚える
  (Variables|Default|SetIntract_Character OtherActor)
  (bind _asgame_flag (Utilities|Casting|CastToGameFlag (Game|GetGameInstance)))
  (Variables|Default|SetAs%20Game%20Flag _asgame_flag))

(fn ConstructionScript
  (|CallParentFunction))