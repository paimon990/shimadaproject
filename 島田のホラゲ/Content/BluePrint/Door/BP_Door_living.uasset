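; Living-room double door that the player opens and closes and BP_Creature can open, gated by GameFlag's DoorKitchenUnlocked.
; Overlap stores the interacting character; DoorOpen toggles a FlipFlop timeline swinging mirrored leaves from BeginPlay yaw, collision off while moving, and turns the knobs.
; DoorOpenC waits briefly, then plays the swing if the FlipFlop reads closed.
; When locked, the player's attempt triggers a DoOnce-guarded rattle of leaves and handles with sound.
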(event Custom|Locked
  ;[1 1 1] Lock時ガチャガチャ
  (Utilities|FlowControl|DoOnce false
    (:Completed
      (Utilities|FlowControl|Sequence
        (:then_0
          (Audio|SpawnSoundatLocation "/Game/SoundEffect/Free_SE/Door_Locked.Door_Locked" (Transformation|GetSocketLocation (Variables|Default|GetDefaultSceneRoot) "None") "0, 0, 0" 1.0 1.0 0.0 0 0)
          (Utilities|FlowControl|Delay 1.5)
          (CallFunction|SoundReset))
        (:then_1
          (bind _ガチャガチャ (Timeline|取っ手ガチャガチャ PlayFromStart)
            (:Update
              (Transformation|SetRelativeRotation (Variables|Default|GetSphere) (Math|Rotator|MakeRotator _ガチャガチャ 0.0 0.0) false false))))
        (:then_2
          (bind _ガチャガチャ_2 (Timeline|取っ手ガチャガチャ2 PlayFromStart)
            (:Update
              (Transformation|SetRelativeRotation (Variables|Default|GetSphere1) (Math|Rotator|MakeRotator _ガチャガチャ_2 0.0 0.0) false false))))
        (:then_3
          (Utilities|FlowControl|Sequence
            (:then_0
              (bind _0_90 (Timeline|ドアガチャガチャ PlayFromStart)
                (:Update
                  (Transformation|SetRelativeRotation (Variables|Default|GetCube) (Math|Rotator|MakeRotator 0.0 0.0 _0_90) false false))))
            (:then_1
              (bind _0_90_2 (Timeline|ドアガチャガチャ2 PlayFromStart)
                (:Update
                  (Transformation|SetRelativeRotation (Variables|Default|GetCube1) (Math|Rotator|MakeRotator 0.0 0.0 _0_90_2) false false))))))))))

(event Custom|Sound_Reset
  ;[1 1 1] Lock時ガチャガチャ
  (Utilities|FlowControl|DoOnce false) ; enters at Reset
)

(event EventDoorOpen
  (bind _default_rotation (Variables|Default|GetDefault_Rotation))
  ;[1 1 1] 誰がOpenイベントを始めたのか
  (Utilities|Casting|CastToTestCharacter (Variables|Default|GetIntract_Character))
  (if (Variables|/Game/BluePrint/GameFlag/GameFlag.GameFlag_C|GetDoor_Kitchen_Unlocked (Variables|Default|GetAs%20Game%20Flag))
    (Utilities|FlowControl|Sequence
      (:then_0
        (bind _isa (Utilities|FlowControl|FlipFlop)
          (:A
            (bind _180_90 (Timeline|ドアの角度調整 Play) ; 設置角度によって調整必須
              (:Update
                ;[1 1 1] コリジョン設定
                (Collision|SetActorEnableCollision false))
              (:Finished
                (Collision|SetActorEnableCollision true)))
            ;[1 1 1] 現在の角度に合わせて+する
            (Utilities|FlowControl|Sequence
              (:then_0
                (Transformation|SetRelativeRotation (Variables|Default|GetCube) (Math|Rotator|MakeRotator (.roll _default_rotation) (.pitch _default_rotation) (+ (.yaw _default_rotation) _180_90)) false false))
              (:then_1
                (Transformation|SetRelativeRotation (Variables|Default|GetCube1) (Math|Rotator|MakeRotator (.roll _default_rotation) (.pitch _default_rotation) (* (- (+ (.yaw _default_rotation) _180_90) 1.8e+02) -1.0)) false false))))
          (:B
            (Timeline|ドアの角度調整 Reverse))))
      (:then_1
        ;[1 1 1] ドアノブ回転
        (Utilities|FlowControl|FlipFlop
          (:A
            (Utilities|FlowControl|Sequence
              (:then_0
                (bind _180_270 (Timeline|ドアノブ PlayFromStart)
                  (:Update
                    (Transformation|SetRelativeRotation (Variables|Default|GetSphere1) (Math|Rotator|MakeRotator _180_270 0.0 0.0) false false))))
              (:then_1
                (bind _0_90 (Timeline|ドアノブ2 PlayFromStart)
                  (:Update
                    (Transformation|SetRelativeRotation (Variables|Default|GetSphere) (Math|Rotator|MakeRotator _0_90 0.0 0.0) false false)))))))))
    (else
      (CallFunction|Locked))))

(event EventDoorOpenC
  (bind _default_rotation (Variables|Default|GetDefault_Rotation))
  ;[1 1 1] 誰がOpenイベントを始めたのか
  (Utilities|FlowControl|Delay 0.2) ; 必須
  (Utilities|Casting|CastToBP_Creature (Variables|Default|GetIntract_Character))
  (if (Variables|/Game/BluePrint/GameFlag/GameFlag.GameFlag_C|GetDoor_Kitchen_Unlocked (Variables|Default|GetAs%20Game%20Flag))
    (if (not (stale EventDoorOpen _isa)) ; 開いてないならクリーチャーが開ける
      (bind _180_90 (Timeline|ドアの角度調整 Play) ; 設置角度によって調整必須
        (:Update
          ;[1 1 1] コリジョン設定
          (Collision|SetActorEnableCollision false))
        (:Finished
          (Collision|SetActorEnableCollision true)))
      ;[1 1 1] 現在の角度に合わせて+する
      (Utilities|FlowControl|Sequence
        (:then_0
          (Transformation|SetRelativeRotation (Variables|Default|GetCube) (Math|Rotator|MakeRotator (.roll _default_rotation) (.pitch _default_rotation) (+ (.yaw _default_rotation) _180_90)) false false))
        (:then_1
          (Transformation|SetRelativeRotation (Variables|Default|GetCube1) (Math|Rotator|MakeRotator (.roll _default_rotation) (.pitch _default_rotation) (* (- (+ (.yaw _default_rotation) _180_90) 1.8e+02) -1.0)) false false))))))

(event EventBeginPlay
  ;[1 1 1] 本来の角度
  (Variables|Default|SetDefault_Rotation (Transformation|GetActorRotation)))

(event Collision|EventActorEndOverlap
  (params (OtherActor :type Actor%20Object%20Reference))
  ;[1 1 1] 接触したキャラを覚える
  (Variables|Default|SetIntract_Character 0))

(event Collision|EventActorBeginOverlap
  (params (OtherActor :type Actor%20Object%20Reference))
  ;[1 1 1] 接触したキャラを覚える
  (Variables|Default|SetIntract_Character OtherActor)
  (bind _asgame_flag (Utilities|Casting|CastToGameFlag (Game|GetGameInstance)))
  (Variables|Default|SetAs%20Game%20Flag _asgame_flag))

(fn ConstructionScript
  (|CallParentFunction))