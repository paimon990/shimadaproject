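; BP_Handsink is a toggleable hand sink whose Gimmick event runs only if the last actor to overlap the lever is a Character.
; A FlipFlop plays or reverses timelines that rotate the lever and scale the water and splash meshes.
; After a short delay it spawns the running-water sound, or stops it and spawns a shut-off sound.
; A DoOnce makes the player emit a loud noise event at the water only once.
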(event OnComponentBeginOverlap(lever2)
  (params (OverlappedComponent :type Primitive%20Component%20Object%20Reference) (OtherActor :type Actor%20Object%20Reference) (OtherComp :type Primitive%20Component%20Object%20Reference) (OtherBodyIndex :type Integer) (bFromSweep :type Boolean) (SweepResult :type Hit%20Result%20Structure%20%28by%20ref%29))
  ;[1 1 1] レバーに触れているか
  (bind _output_get (Variables|Default|SetOverlap_Actor OtherActor)))

(event EventGimmick
  (bind _returnvalue (Game|GetPlayerCharacter 0))
  (bind __water (Variables|Default|Get%20Water))
  (bind _returnvalue_2 (Transformation|GetSocketLocation __water "None"))
  (Utilities|Casting|CastToCharacter (stale OnComponentBeginOverlap(lever2) _output_get))
  (Utilities|FlowControl|FlipFlop
    (:A
      (Utilities|FlowControl|Sequence
        (:then_0
          ;[1 1 1] レバーの回転
          (bind _0_90 (Timeline|Lever Play)
            (:Update
              (Transformation|SetRelativeRotation (Variables|Default|Getlever2) (Math|Rotator|MakeRotator 0.0 0.0 _0_90) false false))))
        (:then_1
          ;[1 1 1] 水の表示、非表示
          (bind _0_0_0275 (Timeline|Water Play)
            (:Update
              (Transformation|SetRelativeScale3D (Variables|Default|Get%20Water) (Math|Vector|MakeVector _0_0_0275 _0_0_0275 0.34)))))
        (:then_2
          (bind _0_0_11 (Timeline|Splash！ Play)
            (:Update
              (Transformation|SetRelativeScale3D (Variables|Default|GetSplash) (Math|Vector|MakeVector _0_0_11 _0_0_11 _0_0_11)))))
        (:then_3
          (Utilities|FlowControl|Delay 0.2)
          (Variables|Default|SetSound_Set "/Game/SoundEffect/Water_HandSink.Water_HandSink")
          (bind _returnvalue_3 (Audio|SpawnSoundatLocation (Variables|Default|GetSound_Set) _returnvalue_2 "0, 0, 0" 0.1 1.0 0.0 "/Game/SoundEffect/Sound_Attenuation.Sound_Attenuation" 0 :!label _label))
          (Variables|Default|SetSound _returnvalue_3)
          (Utilities|FlowControl|DoOnce false
            (:Completed
              (Class|Pawn|PawnMakeNoise _returnvalue 15.0 _returnvalue_2 true _returnvalue))))))
    (:B
      (Utilities|FlowControl|Sequence
        (:then_0
          (Timeline|Lever Reverse))
        (:then_1
          (Timeline|Water Reverse))
        (:then_2
          (Timeline|Splash！ Reverse))
        (:then_3
          (Utilities|FlowControl|Delay 0.2)
          (Audio|Components|Audio|Stop (Variables|Default|GetSound))
          (Variables|Default|SetSound_Set "/Game/SoundEffect/Water_HandSink_Stop.Water_HandSink_Stop")
          (goto _label))))))

(fn ConstructionScript)