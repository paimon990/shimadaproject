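; BP_Light is a flashlight item that highlights when the player can interact and records its pickup.
; Begin and end overlap with TestCharacter share one FlipFlop, toggling the mesh between highlight and normal materials rather than setting each explicitly.
; EndPlay sets FlashLightGot on the GameFlag game instance, so any end of play, not only a pickup, marks the flashlight as obtained.
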(event Collision|EventActorBeginOverlap
  (params (OtherActor :type Actor%20Object%20Reference))
  ;[1 1 1] インタラクト可能時、色を変える
  (Utilities|Casting|CastToTestCharacter OtherActor)
  (Utilities|FlowControl|FlipFlop
    (:A
      (Variables|Default|SetMaterial "/Game/OfficeScene/Materials/M_Item_Light.M_Item_Light"))
    (:B
      (Variables|Default|SetMaterial "/Game/Survival_Items_Pack/Materials/Objects/MI_Flashlight_Small_01.MI_Flashlight_Small_01")))
  (Rendering|Material|SetMaterial (Variables|Default|GetFlashLight) 0 (Variables|Default|GetMaterial)))

(event Collision|EventActorEndOverlap
  (params (OtherActor :type Actor%20Object%20Reference))
  ;[1 1 1] インタラクト可能時、色を変える
  (Utilities|Casting|CastToTestCharacter (stale Collision|EventActorBeginOverlap OtherActor))
  (Utilities|FlowControl|FlipFlop
    (:A
      (Variables|Default|SetMaterial "/Game/OfficeScene/Materials/M_Item_Light.M_Item_Light"))
    (:B
      (Variables|Default|SetMaterial "/Game/Survival_Items_Pack/Materials/Objects/MI_Flashlight_Small_01.MI_Flashlight_Small_01")))
  (Rendering|Material|SetMaterial (Variables|Default|GetFlashLight) 0 (Variables|Default|GetMaterial)))

(event EventEndPlay
  (params (EndPlayReason :type EEndPlayReason%20Enum :default "Destroyed"))
  ;[1 1 1] 消えたらフラッシュライトゲットフラグ立てる
  (bind _asgame_flag (Utilities|Casting|CastToGameFlag (Game|GetGameInstance)))
  (Variables|/Game/BluePrint/GameFlag/GameFlag.GameFlag_C|SetFlash_Light_Got _asgame_flag true))

(fn ConstructionScript
  (|CallParentFunction))