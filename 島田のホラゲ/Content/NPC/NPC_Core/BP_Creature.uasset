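; BP_Creature is an enemy NPC that hunts the player and loads GameOverMap when its capsule touches TestCharacter.
; Capsule overlaps also set the blackboard flag Point_Rotation_Now according to whether the other actor is a rotate point.
; When NPC_Search overlaps a door, it calls DoorOpenC on every door of that class in the level.
; Tick reads the Player_Chase blackboard flag to switch between slow and fast movement speed and acceleration.
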(event OnComponentBeginOverlap(NPC_Search)
  (params (OverlappedComponent :type Primitive%20Component%20Object%20Reference) (OtherActor :type Actor%20Object%20Reference) (OtherComp :type Primitive%20Component%20Object%20Reference) (OtherBodyIndex :type Integer) (bFromSweep :type Boolean) (SweepResult :type Hit%20Result%20Structure%20%28by%20ref%29))
  ;[1 1 1] Doorすべてを取得
  (bind _asbp_door_default (Utilities|Casting|CastToBP_Door_DefaultClass (Utilities|GetClass OtherActor)))
  (bind _outactors (Actor|GetAllActorsOfClass _asbp_door_default))
  (bind _output_get (Variables|Default|SetDoor_Actors _outactors))
  ;[1 1 1] DoorすべてでOpenイベント始動
  (for _index (range 0 (- (Utilities|Array|Length _output_get) 1))
    (Default|DoorOpenC (Utilities|Array|Get(acopy) _output_get _index))))

(event OnComponentBeginOverlap(CapsuleComponent)
  (params (OverlappedComponent :type Primitive%20Component%20Object%20Reference) (OtherActor :type Actor%20Object%20Reference) (OtherComp :type Primitive%20Component%20Object%20Reference) (OtherBodyIndex :type Integer) (bFromSweep :type Boolean) (SweepResult :type Hit%20Result%20Structure%20%28by%20ref%29))
  (Variables|Default|SetOverlap_Actor_A OtherActor)
  (Utilities|FlowControl|Sequence
    (:then_0
      ;[1 1 1] 主人公に触れたらゲームオーバー
      (Utilities|Casting|CastToTestCharacter (Variables|Default|GetOverlap_Actor_A))
      (Game|OpenLevel(byName) "GameOverMap"))
    (:then_1
      ;[1 1 1] RotatoPointにいる場合、今いるポイントの向きを送る
      (Utilities|Casting|CastToBP_RotatePointClass (Utilities|GetClass (Variables|Default|GetOverlap_Actor_A))
        (:then
          (AI|Components|Blackboard|SetValueasBool (AI|GetBlackboard (Pawn|GetController)) (Utilities|Name|MakeLiteralName "Point_Rotation_Now") true))
        (:CastFailed
          (AI|Components|Blackboard|SetValueasBool (AI|GetBlackboard (Pawn|GetController)) (Utilities|Name|MakeLiteralName "Point_Rotation_Now") false))))))

(event EventTick
  (params (DeltaSeconds :type Float%20%28single-precision%29))
  (bind _charactermovement (Variables|Character|GetCharacterMovement))
  ;[1 1 1] 状態によって速度変更
  (if (ScalableFloat|GetValueasBool (AI|GetBlackboard (Pawn|GetController)) (Utilities|Name|MakeLiteralName "Player_Chase"))
    (Variables|/Script/Engine.CharacterMovementComponent|SetMaxWalkSpeed _charactermovement 4.5e+02)
    (Variables|/Script/Engine.CharacterMovementComponent|SetMaxAcceleration _charactermovement 1024.0)
    (else
      (Variables|/Script/Engine.CharacterMovementComponent|SetMaxWalkSpeed _charactermovement 2e+02)
      (Variables|/Script/Engine.CharacterMovementComponent|SetMaxAcceleration _charactermovement 2e+02))))

(fn ConstructionScript)